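; Zombie enemy Blueprint that randomizes its variant when play begins.
; RandomZombieType picks one of four animation Blueprints, including a crawler, each paired with a walk speed and health, trading speed for toughness.
; BeginPlay calls the parent, then applies the result to the mesh's anim class, the movement component's max walk speed and SetHealth.
; The RL and LL variants share the same middle-tier stats.
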(event EventBeginPlay
  (|CallParentFunction)
  (bind (_randomanim _speed _health) (CallFunction|RandomZombieType))
  (Class|SkeletalMeshComponent|SetAnimClass (Variables|Character|GetMesh) _randomanim)
  (Variables|/Script/Engine.CharacterMovementComponent|SetMaxWalkSpeed (Variables|Character|GetCharacterMovement) _speed)
  (Class|EnemyBase|SetHealth _health))

(fn ConstructionScript)

(fn RandomZombieType
  (Utilities|FlowControl|Sequence
    (:then_0
      (switch int (Math|Random|RandomIntegerinRange 0 3)
        (:0
          (LocalVariables|SetAnimPicked "/Game/Animations/AnimBlueprints/ABP_Zombie_BL.ABP_Zombie_BL_C")
          (LocalVariables|SetSpeedPicked 7e+02)
          (LocalVariables|SetHealthPicked 5e+01))
        (:1
          (LocalVariables|SetAnimPicked "/Game/Animations/AnimBlueprints/ABP_Zombie_RL.ABP_Zombie_RL_C")
          (LocalVariables|SetSpeedPicked 5e+02 :!label _label)
          (LocalVariables|SetHealthPicked 1e+02))
        (:2
          (LocalVariables|SetAnimPicked "/Game/Animations/AnimBlueprints/ABP_Zombie_LL.ABP_Zombie_LL_C")
          (goto _label))
        (:3
          (LocalVariables|SetAnimPicked "/Game/Animations/AnimBlueprints/ABP_Zombie_Crawl.ABP_Zombie_Crawl_C")
          (LocalVariables|SetSpeedPicked 3e+02)
          (LocalVariables|SetHealthPicked 1.5e+02))))
    (:then_1
      (return (LocalVariables|GetAnimPicked) (LocalVariables|GetSpeedPicked) (LocalVariables|GetHealthPicked)))))